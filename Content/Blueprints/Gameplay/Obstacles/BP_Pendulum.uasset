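; A swinging pendulum obstacle that knocks players away on contact.
; A timeline, played at a configurable speed from a random start position, rolls the actor back and forth between two angles.
; When the sphere overlaps a Fall Guy character, it applies a velocity-change impulse pushing the character away from the sphere's center, scaled by a push force.
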(event OnComponentBeginOverlap(Sphere)
  (params (OverlappedComponent :type Primitive%20Component%20Object%20Reference) (OtherActor :type Actor%20Object%20Reference) (OtherComp :type Primitive%20Component%20Object%20Reference) (OtherBodyIndex :type Integer) (bFromSweep :type Boolean) (SweepResult :type Hit%20Result%20Structure%20%28by%20ref%29))
  (bind _asbp_fall_guy_character (Utilities|Casting|CastToBP_FallGuyCharacter OtherActor))
  (Physics|AddImpulse (Variables|/Script/Engine.Character|GetCharacterMovement _asbp_fall_guy_character) (* (Math|Vector|GetUnitDirection(Vector) (Transformation|GetWorldLocation (Variables|Default|GetSphere)) (Transformation|GetActorLocation _asbp_fall_guy_character)) (Variables|Default|GetPushForce)) true))

(event EventBeginPlay
  (bind _pendulumtimeline (Variables|Default|GetPendulumTimeline))
  (Components|Timeline|SetPlayRate _pendulumtimeline (Variables|Default|GetpendulumSpeed))
  (Components|Timeline|SetPlaybackPosition _pendulumtimeline (Math|Random|RandomFloat) false true)
  (bind _alpha (Timeline|PendulumTimeline Play)
    (:Update
      (Transformation|SetActorRotation (Math|Rotator|MakeRotator (Math|Float|Lerp 4e+01 -4e+01 _alpha) 0.0 0.0) true))))

(fn ConstructionScript)